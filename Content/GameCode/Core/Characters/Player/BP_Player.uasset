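; BP_Player is the player Blueprint, adjusting the spring arm camera distance while sprinting.
; BeginPlay caches the spring arm's starting length as the default.
; Sprint start plays a timeline that lerps the arm toward the sprint length, and sprint end reverses that timeline to ease it back.
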(event `self.ReceiveBeginPlay`
  (set `self.DefaultSprintArmLenght` (`SpringArmComponent.TargetArmLength` (`self.SpringArmComponent`))))

(event `self.OnSprintStart`
  (bind (_direction _value) (`Timeline|SpringArmSprintTimeline` :!label _label)
    (:`Update`
      (set `SpringArmComponent.TargetArmLength` (`KismetMathLibrary.Lerp` (`self.DefaultSprintArmLenght`) (`self.SprintArmLenght`) _value) (`self.SpringArmComponent`)))))

(event `self.OnSprintEnd`
  (goto _label :!via `Reverse`))

(fn `UserConstructionScript`)